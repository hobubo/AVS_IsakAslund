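; BP_PathActor is an activatable actor that spawns an actor of a configurable class and moves it along a spline.
; On activation it spawns the actor at the spline start, if none exists, and enables tick, which advances distance by Speed and applies the spline transform.
; Tick turns off at the spline's end.
; Reset disables tick, zeroes the distance and teleports the actor back to the start.
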(event Custom|MoveActorAlongSpline
  (params (Delta%20Seconds :type Float%20%28double-precision%29))
  (bind _output_get (Variables|Default|SetDistanceAlongSpline (+ (Variables|Default|GetDistanceAlongSpline) (* Delta%20Seconds (Variables|Default|GetSpeed)))))
  (Transformation|SetWorldTransform (Variables|/Script/Engine.Actor|GetRootComponent (Variables|Default|GetActor)) (Spline|GetTransformatDistanceAlongSpline (Variables|Default|GetSpline) _output_get "World" false) false false)
  (if (>= (Variables|Default|GetDistanceAlongSpline) (Spline|GetSplineLength (Variables|Default|GetSpline)))
    (Actor|Tick|SetActorTickEnabled false)))

(event Custom|SpawnActor
  (Utilities|IsValid (Variables|Default|GetActor)
    (:Is%20Not%20Valid
      (bind _returnvalue (Game|SpawnActorfromClass (Variables|Default|GetActor%20Class) (Spline|GetTransformatDistanceAlongSpline (Variables|Default|GetSpline) 0.0 "World" false) "Undefined" "MultiplyWithRoot" 0 0))
      (Variables|Default|SetActor _returnvalue))))

(event Custom|Reset
  (Actor|Tick|SetActorTickEnabled false)
  (bind _output_get (Variables|Default|SetDistanceAlongSpline 0.0))
  (Utilities|IsValid (Variables|Default|GetActor)
    (:Is%20Valid
      (Transformation|SetActorTransform (Variables|Default|GetActor) (Spline|GetTransformatDistanceAlongSpline (Variables|Default|GetSpline) _output_get "World" false) false true))))

(event EventOnReset
  (Development|PrintString "on r3eset")
  (CallFunction|Reset))

(event EventTick
  (params (DeltaSeconds :type Float%20%28single-precision%29))
  (Utilities|IsValid (Variables|Default|GetActor)
    (:Is%20Valid
      (CallFunction|MoveActorAlongSpline DeltaSeconds))))

(event EventOnActivate
  (params (Activator :type Actor%20Object%20Reference))
  (CallFunction|SpawnActor)
  (Actor|Tick|SetActorTickEnabled true))

(fn ConstructionScript)