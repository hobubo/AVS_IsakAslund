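; A trigger volume that takes movement control from an overlapping actor, auto-runs it forward through the volume and launches a jump on exit.
; On entry it blocks move input and starts a looping timer that steers the actor toward a point ahead of the volume's bounds along its forward vector.
; On exit it triggers the jump and slow motion, then restores speed and input and clears the timer after a delay.
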(event Custom|AutoRunTick
  (bind (_origin _boxextent) (Collision|GetActorBounds false false))
  (Class|IControllable|OnMove(Message) (Variables|Default|GetOther%20Actor) (Math|Vector|GetUnitDirection(Vector) (Transformation|GetActorLocation (Variables|Default|GetOther%20Actor)) (+ _origin (* (.x _boxextent) 2 (Transformation|GetActorForwardVector)))) true))

(event Collision|EventActorBeginOverlap
  (params (OtherActor :type Actor%20Object%20Reference))
  (bind _output_get (Variables|Default|SetOther%20Actor OtherActor))
  (Class|IControllable|SetIgnorMoveInput(Message) _output_get true)
  (bind _returnvalue (Utilities|Time|SetTimerbyEvent (EventDispatchers|CreateEvent :!event Custom|AutoRunTick) 0.01 true))
  (Variables|Default|SetAutoRunTimerHandle _returnvalue))

(event Collision|EventActorEndOverlap
  (params (OtherActor :type Actor%20Object%20Reference))
  (Class|IControllable|OnJump(Message) OtherActor)
  (CallFunction|SetSlowMotion true)
  (Utilities|FlowControl|Delay (Variables|Default|GetReturn%20Controll%20Duration))
  (CallFunction|SetSlowMotion false)
  (Class|IControllable|SetIgnorMoveInput(Message) OtherActor false)
  (Utilities|Time|ClearandInvalidateTimerbyHandle (Variables|Default|GetAutoRunTimerHandle)))

(fn ConstructionScript)