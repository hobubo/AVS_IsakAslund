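; BP_Plane is a flyable plane that takes over player control when an actor overlaps it.
; Overlap attaches the player character to the cockpit socket, blends the view, then possesses the plane and enables Tick.
; Tick moves it constantly forward and lerps roll from look input, which also steers yaw and pitch.
; Shoot toggles a looping timer that spawns bullets alternately from two arrow components.
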(event Custom|AttachPlayerToPlane
  (bind _returnvalue (Game|GetPlayerCharacter 0))
  (Pawn|Components|CharacterMovement|SetMovementMode (Variables|/Script/Engine.Character|GetCharacterMovement _returnvalue) "MOVE_None" 0)
  (Transformation|AttachComponentToComponent _returnvalue (Variables|Default|GetPlane_Mesh) "cockpit" "SnapToTarget" "SnapToTarget" "KeepWorld" true))

(event Custom|Possess
  (bind _returnvalue (Game|GetPlayerController 0))
  (Game|Player|SetViewTargetwithBlend _returnvalue self 1.0 "VTBlend_Linear" 0.0 false)
  (Utilities|FlowControl|Delay 1.0)
  (Pawn|Possess _returnvalue self)
  (Actor|Tick|SetActorTickEnabled true))

(event Custom|AddRollWhenTurning
  (bind _returnvalue (Transformation|GetActorRotation))
  (bind (_roll _pitch _yaw) (Math|Rotator|BreakRotator _returnvalue))
  (Pawn|SetControlRotation (Pawn|GetController) (Math|Rotator|MakeRotator (Math|Float|Lerp _roll (* (.x (Input|EnhancedActionValues|GetIA_Look)) 5.0) 0.05) _pitch _yaw)))

(event Custom|AutoFire
  (Game|SpawnActorfromClass (Variables|Default|GetBullet) (Transformation|GetWorldTransform (Variables|Default|GetArrow)) "Undefined" "MultiplyWithRoot" 0 0)
  (Utilities|FlowControl|Delay (Variables|Default|GetAutoFireInterval))
  (Game|SpawnActorfromClass (Variables|Default|GetBullet) (Transformation|GetWorldTransform (Variables|Default|GetArrow1)) "Undefined" "MultiplyWithRoot" 0 0))

(event Custom|MoveForward
  (params (Delta%20Seconds :type Float%20%28double-precision%29))
  (Transformation|AddActorWorldOffset (* Delta%20Seconds (Variables|Default|GetSpeed) (Transformation|GetActorForwardVector))))

(event EventOnShoot
  (if (Utilities|Time|IsValidTimerHandle (Variables|Default|GetAutoFireTimerHandle))
    (Utilities|Time|ClearandInvalidateTimerbyHandle (Variables|Default|GetAutoFireTimerHandle))
    (else
      (bind _returnvalue (Utilities|Time|SetTimerbyEvent (delegate Custom|AutoFire) (* (Variables|Default|GetAutoFireInterval) 2.0) true))
      (Variables|Default|SetAutoFireTimerHandle _returnvalue))))

(event Collision|EventActorBeginOverlap
  (params (OtherActor :type Actor%20Object%20Reference))
  (Collision|SetActorEnableCollision OtherActor false)
  (CallFunction|AttachPlayertoPlane)
  (CallFunction|Possess))

(event EventOnLook
  (params (Input :type Vector%202D%20Structure))
  (Pawn|Input|AddControllerYawInput (/ (.x Input) 5.0))
  (Pawn|Input|AddControllerPitchInput (/ (.y Input) 5.0)))

(event EventTick
  (params (DeltaSeconds :type Float%20%28single-precision%29))
  (CallFunction|MoveForward DeltaSeconds)
  (CallFunction|AddRollwhenTurning))

(fn ConstructionScript)