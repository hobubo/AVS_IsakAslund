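; Player controller that turns Enhanced Input into movement, look, jump and shoot messages for the possessed pawn.
; BeginPlay adds the input mapping context, creates a hidden pause menu widget and sets game-only input; the pause action toggles that menu.
; Move input is made camera-relative using the camera manager's right and forward vectors, flattened to the horizontal plane.
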(event Input|EnhancedActionEvents|EnhancedInputActionIA_Look
  (params (ActionValue :type Vector%202D%20Structure) (ElapsedSeconds :type Float%20%28double-precision%29) (TriggeredSeconds :type Float%20%28double-precision%29) (InputAction :type Input%20Action%20Object%20Reference :default "/Game/Player/Input/IA_Look.IA_Look"))
  (Class|IControllable|OnLook(Message) (Variables|Default|GetTarget) ActionValue))

(event Input|EnhancedActionEvents|EnhancedInputActionIA_Jump
  (params (ActionValue :type Boolean) (ElapsedSeconds :type Float%20%28double-precision%29) (TriggeredSeconds :type Float%20%28double-precision%29) (InputAction :type Input%20Action%20Object%20Reference :default "/Game/Player/Input/IA_Jump.IA_Jump"))
  (Class|IControllable|OnJump(Message) (Variables|Default|GetTarget)))

(event Input|EnhancedActionEvents|EnhancedInputActionIA_Shoot
  (params (ActionValue :type Boolean) (ElapsedSeconds :type Float%20%28double-precision%29) (TriggeredSeconds :type Float%20%28double-precision%29) (InputAction :type Input%20Action%20Object%20Reference :default "/Game/Player/Input/IA_Shoot.IA_Shoot"))
  (Class|IControllable|OnShoot(Message) (Variables|Default|GetTarget)))

(event Input|EnhancedActionEvents|EnhancedInputActionIA_Pause
  (params (ActionValue :type Boolean) (ElapsedSeconds :type Float%20%28double-precision%29) (TriggeredSeconds :type Float%20%28double-precision%29) (InputAction :type Input%20Action%20Object%20Reference :default "/Game/Player/Input/IA_Pause.IA_Pause"))
  (Default|TogglePause (Variables|Default|GetPauseMenu)))

(event Input|EnhancedActionEvents|EnhancedInputActionIA_Move
  (params (ActionValue :type Vector%202D%20Structure) (ElapsedSeconds :type Float%20%28double-precision%29) (TriggeredSeconds :type Float%20%28double-precision%29) (InputAction :type Input%20Action%20Object%20Reference :default "/Game/Player/Input/IA_Move.IA_Move"))
  (Class|IControllable|OnMove(Message) (Variables|Default|GetTarget) (|TranslateVectorByActiveCamera_2 (.x ActionValue) (.y ActionValue)) false))

(event EventPossess
  (params (PossessedPawn :type Pawn%20Object%20Reference))
  (Variables|Default|SetTarget PossessedPawn))

(event EventBeginPlay
  (Input|AddMappingContext)
  (|CreatePauseMenu)
  (Input|SetInputModeGameOnly self false))

(fn ConstructionScript)