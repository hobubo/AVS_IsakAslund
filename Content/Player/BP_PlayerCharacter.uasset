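; Player character Blueprint that handles Enhanced Input actions for move, look and jump.
; Look input drives controller yaw and pitch, and jump calls the built-in Jump.
; Move passes input through TranslateVectorByActiveCamera to get the movement direction.
; That helper builds a normalized, flattened vector from the active camera's right and forward axes, but the graph shows this result as unused.
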(event Input|EnhancedActionEvents|EnhancedInputActionIA_Move
  (params (ActionValue :type Vector%202D%20Structure) (ElapsedSeconds :type Float%20%28double-precision%29) (TriggeredSeconds :type Float%20%28double-precision%29) (InputAction :type Input%20Action%20Object%20Reference :default "/Game/Player/Input/IA_Move.IA_Move"))
  (Pawn|Input|AddMovementInput (|TranslateVectorByActiveCamera (.x ActionValue) (.y ActionValue)) 1.0 false))

(event Input|EnhancedActionEvents|EnhancedInputActionIA_Look
  (params (ActionValue :type Vector%202D%20Structure) (ElapsedSeconds :type Float%20%28double-precision%29) (TriggeredSeconds :type Float%20%28double-precision%29) (InputAction :type Input%20Action%20Object%20Reference :default "/Game/Player/Input/IA_Look.IA_Look"))
  (Pawn|Input|AddControllerYawInput (.x ActionValue))
  (Pawn|Input|AddControllerPitchInput (.y ActionValue)))

(event Input|EnhancedActionEvents|EnhancedInputActionIA_Jump
  (params (ActionValue :type Boolean) (ElapsedSeconds :type Float%20%28double-precision%29) (TriggeredSeconds :type Float%20%28double-precision%29) (InputAction :type Input%20Action%20Object%20Reference :default "/Game/Player/Input/IA_Jump.IA_Jump"))
  (Character|Jump))

(fn ConstructionScript)